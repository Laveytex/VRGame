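; BP_Enemy_01 is an enemy character that shows its health as floating text and spawns damage numbers when hit.
; Each tick it writes current health to a TextRender and destroys that component once health reaches zero.
; FindRotation computes a yaw-only look-at toward the VRPawn, stored as TextRotation.
; On damage, it spawns BP_FloatingText above the health text with that rotation and the negated damage value.
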(event `self.ReceiveTick`
  (params (DeltaSeconds :type "Float (single-precision)"))
  (bind _currenhealth (`self.CurrenHealth`))
  (`/Engine/EditorBlueprintResources/StandardMacros.IsValid` (`self.TextRender`)
    (:`Is Valid`
      (if (<= _currenhealth 0.0)
        (`ActorComponent.K2_DestroyComponent` (`self.TextRender`))
        (else
          (`self.FindRotation`)
          (`TextRenderComponent.K2_SetText` (`self.TextRender`) (`KismetTextLibrary.Conv_DoubleToText` _currenhealth "HalfToEven")))))))

(event `self.OnTakeDamage`
  (params (Damage :type "Float (single-precision)"))
  (bind _returnvalue_location (`KismetMathLibrary.BreakTransform` (`SceneComponent.K2_GetComponentToWorld` (`self.TextRender`))))
  (`|SpawnActorFromClass` "/Game/my/Blueprint/UI/BP_FloatingText.BP_FloatingText_C" (`KismetMathLibrary.MakeTransform` (+ _returnvalue_location (0.0 0.0 50.0)) (`self.TextRotation`)) "AlwaysSpawn" "OverrideRootScale" null (`KismetTextLibrary.Conv_StringToText` (`KismetStringLibrary.Concat_StrStr` "-" (`KismetTextLibrary.Conv_TextToString` (`KismetTextLibrary.Conv_DoubleToText` Damage "HalfToEven")))) null))

(event `FindRotation`
  (bind _returnvalue (`GameplayStatics.GetActorOfClass` "/Game/VRTemplate/Blueprints/VRPawn.VRPawn_C"))
  (`/Engine/EditorBlueprintResources/StandardMacros.IsValid` _returnvalue
    (:`Is Valid`
      (bind (_returnvalue_roll _returnvalue_pitch _returnvalue_yaw) (`KismetMathLibrary.BreakRotator` (`KismetMathLibrary.FindLookAtRotation` (`SceneComponent.K2_GetComponentLocation` (`self.TextRender`)) (`self.K2_GetActorLocation` _returnvalue))))
      (set `self.TextRotation` (`KismetMathLibrary.MakeRotator` 0.0 0.0 _returnvalue_yaw)))
    (:`Is Not Valid`
      (set `self.TextRotation` (struct)))))

(fn `UserConstructionScript`)