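; BP_DamagValuem is a damage volume that hurts the VR player while they stand inside its box.
; Overlapping actors that implement DamageTakerInterface set IsIn, and a VRPawn among them starts SetDamage, which applies fixed Health damage in a Delay loop.
; Any actor leaving the box clears IsIn, which ends the loop.
; Each tick, FindRotation turns the TextRender label on yaw only to face the VRPawn.
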(event `SetDamage`
  (params (Actor :type "/Game/VRTemplate/Blueprints/VRPawn Object Reference"))
  (`/Engine/EditorBlueprintResources/StandardMacros.IsValid` Actor :!label _label
    (:`Is Valid`
      (if (`self.IsIn`)
        (`HealthComponent.TakeDamage` (`/Game/VRTemplate/Blueprints/VRPawn.Health` Actor) 10)
        (`KismetSystemLibrary.Delay` 0.5)
        (goto _label)))))

(event `self.ReceiveTick`
  (params (DeltaSeconds :type "Float (single-precision)"))
  (`self.FindRotation`)
  (`SceneComponent.K2_SetRelativeRotation` (`self.TextRender`) (`self.TextRotation`) false false))

(event `self.Box.OnComponentBeginOverlap`
  (params (OverlappedComponent :type "PrimitiveComponent Object Reference") (OtherActor :type "Actor Object Reference") (OtherComp :type "PrimitiveComponent Object Reference") (OtherBodyIndex :type Integer) (bFromSweep :type Boolean) (SweepResult :type "HitResult Structure (by ref)"))
  (if (`KismetSystemLibrary.DoesImplementInterface` OtherActor "/Script/VRGamePreview.DamageTakerInterface")
    (set `self.IsIn` true)
    (bind _asvrpawn (cast `/Game/VRTemplate/Blueprints/VRPawn` OtherActor))
    (`self.SetDamage` _asvrpawn)))

(event `self.Box.OnComponentEndOverlap`
  (params (OverlappedComponent :type "PrimitiveComponent Object Reference") (OtherActor :type "Actor Object Reference") (OtherComp :type "PrimitiveComponent Object Reference") (OtherBodyIndex :type Integer))
  (set `self.IsIn` false))

(event `FindRotation`
  (bind _returnvalue (`GameplayStatics.GetActorOfClass` "/Game/VRTemplate/Blueprints/VRPawn.VRPawn_C"))
  (`/Engine/EditorBlueprintResources/StandardMacros.IsValid` _returnvalue
    (:`Is Valid`
      (bind (_returnvalue_roll _returnvalue_pitch _returnvalue_yaw) (`KismetMathLibrary.BreakRotator` (`KismetMathLibrary.FindLookAtRotation` (`SceneComponent.K2_GetComponentLocation` (`self.TextRender`)) (`self.K2_GetActorLocation` _returnvalue))))
      (set `self.TextRotation` (`KismetMathLibrary.MakeRotator` 0.0 0.0 _returnvalue_yaw)))
    (:`Is Not Valid`
      (set `self.TextRotation` (struct)))))

(fn `UserConstructionScript`)