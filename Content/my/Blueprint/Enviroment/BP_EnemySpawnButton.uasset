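; BP_EnemySpawnButton is a VR push button that triggers SpawnEnemy on every BP_SpawnEnemyPoint in the level.
; A VRPawn overlapping the Box plays a sound and a Timeline that incrementally offsets InteractBody along relative Y.
; SpawnBlock prevents retriggering until the Timeline finishes.
; The flag is set before the pawn cast, so a non-VRPawn overlap leaves the button blocked.
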(event `self.ReceiveBeginPlay`)

(event `SpawnEnemy`
  (bind _outactors (`GameplayStatics.GetAllActorsOfClass` "/Game/my/Blueprint/Enviroment/BP_SpawnEnemyPoint.BP_SpawnEnemyPoint_C"))
  (for _array_element _outactors
    (`/Game/my/Blueprint/Enviroment/BP_SpawnEnemyPoint.SpawnEnemy` _array_element)))

(event `self.ReceiveActorBeginOverlap`
  (params (OtherActor :type "Actor Object Reference")))

(event `ButtonPushed`
  (bind _interactbody (`self.InteractBody`))
  (bind (_relativelocation_x _relativelocation_y _relativelocation_z) (`KismetMathLibrary.BreakVector` (`SceneComponent.RelativeLocation` _interactbody)))
  (`GameplayStatics.PlaySound2D` "/Engine/EditorSounds/GamePreview/EndSimulate_Cue.EndSimulate_Cue" 1.0 1.0 0.0 null null)
  (bind (_direction _position) (`Timeline|Timeline_0`)
    (:`Update`
      (`SceneComponent.K2_SetRelativeLocation` _interactbody (`KismetMathLibrary.MakeVector` _relativelocation_x (+ _relativelocation_y (* _position 0.1)) _relativelocation_z) false false))
    (:`Finished`
      (set `self.SpawnBlock` false))))

(event `self.Box.OnComponentBeginOverlap`
  (params (OverlappedComponent :type "PrimitiveComponent Object Reference") (OtherActor :type "Actor Object Reference") (OtherComp :type "PrimitiveComponent Object Reference") (OtherBodyIndex :type Integer) (bFromSweep :type Boolean) (SweepResult :type "HitResult Structure (by ref)"))
  (if (not (`self.SpawnBlock`))
    (set `self.SpawnBlock` true)
    (cast `/Game/VRTemplate/Blueprints/VRPawn` OtherActor)
    (`self.ButtonPushed`)
    (`self.SpawnEnemy`)))

(fn `UserConstructionScript`)